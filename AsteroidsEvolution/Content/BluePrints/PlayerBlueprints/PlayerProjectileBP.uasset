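; PlayerProjectileBP is the player's bullet, which destroys asteroids it overlaps.
; On overlap with a BP_Asteroids actor it enables mesh collision, destroys the asteroid and prints its type.
; Big asteroids then request a Medium spawn and Medium ones a Small spawn through BPAsteRef, whose only assignment in this graph is disconnected.
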(event `self.ReceiveActorBeginOverlap`
  (params (OtherActor :type "Actor Object Reference"))
  (bind _bp_aste_ref (`self.BP_Aste_ref`))
  ;[1 1 1] Bullet behavior
  (bind _asbp_asteroids (cast `/Game/TwinStickBP/Blueprints/BP_Asteroids` OtherActor))
  (`PrimitiveComponent.SetCollisionEnabled` (`self.ProjectileMesh`) "QueryAndPhysics")
  (`self.K2_DestroyActor` _asbp_asteroids)
  (bind _type (`/Game/TwinStickBP/Blueprints/BP_Asteroids.Type` _asbp_asteroids))
  (`KismetSystemLibrary.PrintString` (`|GetEnumeratorNameAsString` _type))
  (switch `/Game/TwinStickBP/Blueprints/Enum_meteorite` _type
    (:`NewEnumerator0`
      (`/Game/TwinStickBP/Blueprints/BP_Asteroids.Spawn_new` _bp_aste_ref "NewEnumerator1"))
    (:`NewEnumerator1`
      (`/Game/TwinStickBP/Blueprints/BP_Asteroids.Spawn_new` _bp_aste_ref "NewEnumerator2"))))

(fn `UserConstructionScript`)