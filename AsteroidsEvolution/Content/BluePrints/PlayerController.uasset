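; Player blueprint for a mouse-steered, thruster-driven body with a camera that follows it in the horizontal plane.
; Each tick it yaws the Player component toward the deprojected mouse ray's horizontal direction, taken from the actor's location.
; Positive MoveForward input applies a constant force along that facing, without delta-time scaling.
; PlayerCam then snaps to the Player's X and Y, keeping its own height.
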(event `self.ReceiveTick`
  (params (DeltaSeconds :type "Float (single-precision)"))
  (bind _playerdir (`self.ChangePlayerRot`))
  (`self.UseBackThruster` _playerdir DeltaSeconds 10000.0)
  (`self.SetCameraPos`))

(fn `ChangePlayerRot`
  (returns (playerDir :type "Vector Structure"))
  (bind _returnvalue (`self.K2_GetActorLocation`))
  (bind _returnvalue_2 (`KismetMathLibrary.FindLookAtRotation` _returnvalue (`KismetMathLibrary.MakeVector` (.x (+ _returnvalue (`.WorldDirection` (`PlayerController.DeprojectMousePositionToWorld` (`GameplayStatics.GetPlayerController` 0))))) (.y (+ _returnvalue (`.WorldDirection` (`PlayerController.DeprojectMousePositionToWorld` (`GameplayStatics.GetPlayerController` 0))))) (.z _returnvalue))))
  (bind _yaw (.yaw _returnvalue_2))
  (`SceneComponent.K2_SetWorldRotation` (`self.Player`) _returnvalue_2 false false)
  (return (`KismetMathLibrary.MakeVector` (`KismetMathLibrary.DegCos` _yaw) (`KismetMathLibrary.DegSin` _yaw))))

(fn `SetCameraPos`
  (`SceneComponent.K2_SetWorldLocation` (`self.PlayerCam`) (`KismetMathLibrary.MakeVector` (.x (`SceneComponent.K2_GetComponentLocation` (`self.Player`))) (.y (`SceneComponent.K2_GetComponentLocation` (`self.Player`))) (.z (`SceneComponent.K2_GetComponentLocation` (`self.PlayerCam`)))) false false))

(fn `UseBackThruster`
  (params (PlayerDir :type "Vector Structure") (deltaTime :type "Float (double-precision)") (Speed :type "Float (double-precision)"))
  (if (> (`self.GetInputAxisValue`) 0.0)
    (`PrimitiveComponent.AddForce` (`self.Player`) (* (`KismetMathLibrary.Normal` PlayerDir) Speed) "None" false)))

(fn `UserConstructionScript`)